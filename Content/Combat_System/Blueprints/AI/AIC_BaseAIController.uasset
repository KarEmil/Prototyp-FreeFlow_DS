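; Base AI controller for enemy pawns that runs each enemy's behavior tree on possession and tracks the player as its target.
; It mirrors the combat component's toggle event into the blackboard.
; Perception updates set the blackboard Target and notify the enemy when either of the first two stimuli senses a Player-tagged actor.
; Losing the first stimulus clears the target, while losing the second does not.
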(event OnPerceptionUpdated(AIPerception)
  (params (UpdatedActors :type Array%20of%20Actor%20Object%20References))
  (CallFunction|UpDatePerception UpdatedActors))

(event Custom|OnToggleCombat
  (params (B_IsCombatEnabled? :type Boolean))
  (AI|Components|Blackboard|SetValueasBool (Variables|Default|GetBlackboard) (Utilities|Name|MakeLiteralName "B_CombatEnabled") B_IsCombatEnabled?))

(event EventPossess
  (params (PossessedPawn :type Pawn%20Object%20Reference))
  (bind _asbp_base_enemis (Utilities|Casting|CastToBP_BaseEnemis PossessedPawn))
  (Variables|Default|SetRef%20Base%20Enemis _asbp_base_enemis)
  (EventDispatchers|BindEventtoOnCombatToggled (Variables|/Game/Combat_System/Blueprints/AI/BP_BaseEnemis.BP_BaseEnemis_C|GetAC_CombatComponent (Variables|Default|GetRef%20Base%20Enemis)) (delegate Custom|OnToggleCombat))
  (AI|RunBehaviorTree (Variables|/Game/Combat_System/Blueprints/AI/BP_BaseEnemis.BP_BaseEnemis_C|GetBehavior%20Tree (Variables|Default|GetRef%20Base%20Enemis))))

(fn ConstructionScript)

(fn UpDatePerception
  (params (PerceivedActor :type Array%20of%20Actor%20Object%20References))
  (for _array_element PerceivedActor
    (LocalVariables|SetL_SenseActor _array_element)
    (bind _info (Class|AIPerceptionComponent|GetActorsPerception (Variables|Default|GetAIPerception) (LocalVariables|GetL_SenseActor)))
    (for (_array_element_2 _array_index) (.LastSensedStimuli (Utilities|Struct|BreakActorPerceptionBlueprintInfo _info))
      (LocalVariables|SetL_AIStimulus _array_element_2)
      (switch int _array_index
        (:0
          (if (.bSuccessfullySensed (Utilities|Struct|BreakAIStimulus (LocalVariables|GetL_AIStimulus)))
            (bind _returnvalue (Class|BPIGameplayTagBlueprintTag|HasMatchingGameplayTag(Message) (LocalVariables|GetL_SenseActor) "(TagName=\"Character.Player\")"))
            (if _returnvalue
              (CallFunction|SetTargetActor (LocalVariables|GetL_SenseActor)))
            (else
              (CallFunction|SetTargetActor))))
        (:1
          (if (.bSuccessfullySensed (Utilities|Struct|BreakAIStimulus (LocalVariables|GetL_AIStimulus)))
            (bind _returnvalue_2 (Class|BPIGameplayTagBlueprintTag|HasMatchingGameplayTag(Message) (LocalVariables|GetL_SenseActor) "(TagName=\"Character.Player\")"))
            (if _returnvalue_2
              (CallFunction|SetTargetActor (LocalVariables|GetL_SenseActor)))))))))

(fn SetTargetActor
  (params (NewActorTarget :type Actor%20Object%20Reference))
  (AI|Components|Blackboard|SetValueasObject (Variables|Default|GetBlackboard) (Utilities|Name|MakeLiteralName "Target") NewActorTarget)
  (bind _ref_base_enemis (Variables|Default|GetRef%20Base%20Enemis)
    (:then
      (Default|OnTargetSet _ref_base_enemis NewActorTarget))
    (:else)))