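; BP_EnemisV1 is an enemy character that extends a parent class with a melee-style weapon mesh and a health bar.
; The health bar widget reads the stats component and shows only while the enemy is targeted.
; Weapon collision hits apply point damage from a stat value to actors that can receive it.
; Toggling combat snaps the weapon between hand and stowed sockets, and death switches it to physics simulation.
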(event OnCombatToggled(AC_CombatComponent)
  (params (B_IsCombatEnabled? :type Boolean))
  (Transformation|AttachComponentToComponent (Variables|Default|GetWeaponMesh) (Variables|Character|GetMesh) (select B_IsCombatEnabled? (Variables|Socket|GetWeapon%20Hand%20Socket%20Name) (Variables|Socket|GetAttach%20Socket%20Name)) "SnapToTarget" "SnapToTarget" "SnapToTarget" true))

(event OnHit(AC_CollisionComponent)
  (params (HitResult :type Hit%20Result%20Structure))
  (bind _hitactor (Collision|BreakHitResult HitResult))
  (bind _returnvalue (Class|BPICombat|CanRecieveDamage(Message) _hitactor))
  (if _returnvalue
    (Game|Damage|ApplyPointDamage _hitactor (Default|GetCurrentStatsValue (Variables|Default|GetAC_StatsComponent) "NewEnumerator4") (Transformation|GetActorForwardVector) HitResult (Pawn|GetController) self "/Game/Combat_System/Blueprints/DamageType/BP_DamageType.BP_DamageType_C")))

(event Custom|SimulateWeaponPHysics
  (bind _weaponmesh (Variables|Default|GetWeaponMesh))
  (Collision|SetCollisionProfileName _weaponmesh "PhysicsActor" true :!class /Script/Engine.PrimitiveComponent)
  (Physics|SetSimulatePhysics _weaponmesh true)
  (Collision|SetCollisionEnabled (Variables|Default|GetWeaponMesh) "PhysicsOnly"))

(event EventBeginPlay
  (|CallParentFunction)
  (Default|SetCollisionMesh (Variables|Default|GetAC_CollisionComponent) (Variables|Default|GetWeaponMesh))
  (bind _returnvalue (UserInterface|CreateWidget "/Game/Combat_System/Blueprints/UI/WB_HealthBar.WB_HealthBar_C" (Game|GetPlayerController 0) (Variables|Default|GetAC_StatsComponent)))
  (UserInterface|SetWidget (Variables|Default|GetHealthBar) _returnvalue))

(event EventPreformDeath
  (|CallParentFunction)
  (CallFunction|SimulateWeaponPHysics))

(event EventOnTarget
  (params (B_IsTarget? :type Boolean))
  (|CallParentFunction B_IsTarget?)
  (Rendering|SetVisibility (Variables|Default|GetHealthBar) B_IsTarget? false))

(fn ConstructionScript
  (|CallParentFunction))