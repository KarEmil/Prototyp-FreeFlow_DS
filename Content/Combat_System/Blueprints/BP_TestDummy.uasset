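; BP_TestDummy is a combat test dummy that the player can lock on to.
; On BeginPlay it initializes its stats component, then spawns and equips each StartingEquipment class with itself as owner and instigator.
; Targeting events toggle its lock-on widget, and it reports as targetable unless its state manager component is in the Death state.
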(event EventBeginPlay
  (bind _self self)
  (Default|InitializeStats (Variables|Default|GetAC_StatsComponent))
  (for _array_element (Variables|initialization|GetStartingEquipment)
    (bind _returnvalue (Game|SpawnActorfromClass _array_element (Transformation|GetActorTransform) "Undefined" "MultiplyWithRoot" _self _self))
    (Default|OnEquip _returnvalue)))

(event Collision|EventActorBeginOverlap
  (params (OtherActor :type Actor%20Object%20Reference)))

(event EventTick
  (params (DeltaSeconds :type Float%20%28single-precision%29)))

(event EventOnTarget
  (params (B_IsTarget? :type Boolean))
  (Rendering|SetVisibility (Variables|Default|GetLockOnWidget) B_IsTarget? false))

(fn ConstructionScript
  (|CallParentFunction))

(fn CanbeTargeted?
  (return (not (Default|IsCurrentStateEqualtoAny? (Variables|Default|GetAC_StateManagerComponent) "(GameplayTags=((TagName=\"Character.State.Death\")))"))))