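; BP_BaseEquippable is a base actor for combat system items that a Character can equip.
; OnEquip sets the IsEquip flag and snaps the item to a named socket on the owning Character's mesh.
; OnUnEquip only clears the flag, without detaching.
; GetItemMesh returns the static mesh component if it has a mesh assigned, otherwise the skeletal one, so items can use either type.
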(event EventBeginPlay)

(event Collision|EventActorBeginOverlap
  (params (OtherActor :type Actor%20Object%20Reference)))

(event EventTick
  (params (DeltaSeconds :type Float%20%28single-precision%29)))

(fn ConstructionScript)

(fn GetItemMesh
  (Utilities|IsValid (Variables|/Script/Engine.StaticMeshComponent|GetStaticMesh (Variables|Components|GetItemStaticMesh))
    (:Is%20Valid
      (return (Variables|Components|GetItemStaticMesh)))
    (:Is%20Not%20Valid
      (return (Variables|Components|GetItemSkeletalMesh)))))

(fn OnEquip
  (Variables|Default|SetIsEquip? true)
  (ItemMesh|AttachActor (Variables|Initialization|Confing|GetAttach%20Socket%20Name)))

(fn OnUnEquip
  (if (Variables|Default|GetIsEquip?)
    (Variables|Default|SetIsEquip? false)))

(fn AttachActor
  (params (SocketName :type Name))
  (Transformation|AttachComponentToComponent (Variables|/Script/Engine.Character|GetMesh (.AsCharacter (Utilities|Casting|CastToCharacter (Components|GetOwner)))) SocketName "SnapToTarget" "SnapToTarget" "SnapToTarget" true))

(fn SetIsEquipped
  (params (IsEquip? :type Boolean))
  (Variables|Default|SetIsEquip? IsEquip?))

(fn IsEquipped?
  (return (Variables|Default|GetIsEquip?)))