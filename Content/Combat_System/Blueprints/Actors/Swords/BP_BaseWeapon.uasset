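; Base weapon actor for melee combat that moves between hand and sheath sockets and deals point damage on hit.
; On equip it registers with the owner's combat component, updates the animation combat type and points its collision component at the item mesh.
; Gameplay tags select action montages, while the current action from the state manager drives stat cost and damage multiplier.
; It can also switch to simulated physics.
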(event OnHit(AC_CollisionComponent)
  (params (HitResult :type Hit%20Result%20Structure))
  (bind _hitactor (Collision|BreakHitResult HitResult))
  (bind _returnvalue (Class|BPICombat|CanRecieveDamage(Message) _hitactor))
  (if _returnvalue
    (Game|Damage|ApplyPointDamage _hitactor (Stat|GetDamage) (Transformation|GetActorForwardVector (Components|GetOwner)) HitResult (Game|GetInstigatorController) self (Variables|Initialization|GetDamage%20Type%20Class))))

(event Custom|Toggle%20Weapon%20Combat
  (params (B_EnableCombat? :type Boolean))
  (CallFunction|AttachActor (select B_EnableCombat? (Variables|Socket|GetHandSocketName) (Variables|Default|GetAttach%20Socket%20Name))))

(event Custom|SimulateWeaponPHysics
  (bind _returnvalue (CallFunction|GetItemMesh))
  (Collision|SetCollisionProfileName _returnvalue "PhysicsActor" true :!class /Script/Engine.PrimitiveComponent)
  (Physics|SetSimulatePhysics _returnvalue true)
  (Collision|SetCollisionEnabled (Variables|Default|GetItemStaticMesh) "PhysicsOnly"))

(event EventBeginPlay
  (|CallParentFunction) ; This node is disabled and will not be called.\nDrag off pins to build functionality.
)

(event Collision|EventActorBeginOverlap
  (params (OtherActor :type Actor%20Object%20Reference))
  (|CallParentFunction OtherActor) ; This node is disabled and will not be called.\nDrag off pins to build functionality.
)

(event EventTick
  (params (DeltaSeconds :type Float%20%28single-precision%29))
  (|CallParentFunction DeltaSeconds) ; This node is disabled and will not be called.\nDrag off pins to build functionality.
)

(fn ConstructionScript
  (|CallParentFunction))

(fn OnEquip
  (bind _ac_collisioncomponent (Variables|Components|GetAC_CollisionComponent))
  (|CallParentFunction)
  (Variables|Default|SetRef_AC_CombatComponent (Actor|GetComponentbyClass (Components|GetOwner) "/Game/Combat_System/Blueprints/Components/AC_CombatComponent.AC_CombatComponent_C"))
  (EventDispatchers|BindEventtoOnCombatToggled (Variables|Default|GetRef_AC_CombatComponent) (EventDispatchers|CreateEvent :!event Custom|Toggle%20Weapon%20Combat))
  (Variables|Default|SetRef_AC_StatsComponent (Actor|GetComponentbyClass (Components|GetOwner) "/Game/Combat_System/Blueprints/Components/AC_StatsComponent.AC_StatsComponent_C"))
  (Variables|Components|SetRef_StateManagerComponent (Actor|GetComponentbyClass (Components|GetOwner) "/Game/Combat_System/Blueprints/Components/AC_StateManagerComponent.AC_StateManagerComponent_C"))
  (Default|AttachActor self (select (Default|GetCombatEnable (Variables|Default|GetRef_AC_CombatComponent)) (Variables|Socket|GetHandSocketName) (Variables|Default|GetAttach%20Socket%20Name)))
  (Default|SetMainWeapon (Variables|Default|GetRef_AC_CombatComponent) self)
  (Class|BPIAnimation|UpdateCombatType(Message) (Components|SkeletalMesh|GetAnimInstance (Variables|/Script/Engine.Character|GetMesh (.AsCharacter (Utilities|Casting|CastToCharacter (Components|GetOwner))))) (Variables|Initialization|GetCombatType))
  (Default|SetCollisionMesh _ac_collisioncomponent (CallFunction|GetItemMesh))
  (Default|AddActortoIgnore _ac_collisioncomponent (Components|GetOwner)))

(fn GetActionMontage
  (params (CurrentAction :type Gameplay%20Tag%20Structure))
  (|SwitchGameplayTag CurrentAction
    (:Character.Action.Attack.ChargeAttack
      (return (Variables|Animation|GetChargeAttackMontage)))
    (:Character.Action.Attack.FallingAttack
      (return (Variables|Animation|GetFallingAttackMontage)))
    (:Character.Action.Attack.HeavyAttack
      (return (Variables|Animation|GetHeavyAttackMontage)))
    (:Character.Action.Attack.LightAttack
      (return (Variables|Animation|GetLightAttackMontage)))
    (:Character.Action.Attack.SprintAttack
      (return (Variables|Animation|GetSprint%20AttackMontage)))
    (:Character.Action.Dodge
      (return (Variables|Animation|GetDodgeMontageMontage)))
    (:Character.Action.EndCombat
      (return (Utilities|Array|MakeArray (Variables|Animation|GetEndCombat))))
    (:Character.Action.EnterCombat
      (return (Utilities|Array|MakeArray (Variables|Animation|GetStartCombat))))
    (:Character.Action.Attack.FinishAttack
      (return (Variables|Animation|GetFinishAttackMontage)))))

(fn GetStatCostforAction
  (bind _ref_statemanagercomponent (Variables|Components|GetRef_StateManagerComponent)
    (:then
      (return (.Value (Utilities|Map|Find (Variables|Stat|GetActionStatCost) (Default|GetCurrentCharacterAction _ref_statemanagercomponent)))))
    (:else
      (return 0.0))))

(fn GetDamage
  (bind _ref_statemanagercomponent (Variables|Components|GetRef_StateManagerComponent)
    (:then
      (return (* (Variables|Stat|GetDamage) (Math|Float|Clamp(Float) (.Value (Utilities|Map|Find (Variables|Default|GetActionDamageMultiplier) (Default|GetCurrentCharacterAction _ref_statemanagercomponent))) 1.0 (.Value (Utilities|Map|Find (Variables|Default|GetActionDamageMultiplier) (Default|GetCurrentCharacterAction _ref_statemanagercomponent)))))))
    (:else
      (return (Variables|Stat|GetDamage)))))

(fn ActivateCollision
  (params (CollisionPart :type E_CollisionPart%20Enum :default "NewEnumerator0"))
  (Default|EnableCollision (Variables|Components|GetAC_CollisionComponent)))

(fn DeactivateCollision
  (params (CollisionPart :type E_CollisionPart%20Enum :default "NewEnumerator0"))
  (Default|DisableCollision (Variables|Components|GetAC_CollisionComponent)))