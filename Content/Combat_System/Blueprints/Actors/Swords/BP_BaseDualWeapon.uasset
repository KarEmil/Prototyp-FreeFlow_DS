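; Base Blueprint for dual-wielded weapons in the combat system, extending its parent weapon with an off-hand piece and a second collision component.
; On equip it assigns the off-hand to the left collision component and snaps it to the owning character's hand or stowed socket based on combat state.
; Toggling combat moves the off-hand between those sockets, while collision activation and deactivation route to main or off-hand by collision part.
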(event EventBeginPlay
  (|CallParentFunction) ; This node is disabled and will not be called.\nDrag off pins to build functionality.
)

(event Collision|EventActorBeginOverlap
  (params (OtherActor :type Actor%20Object%20Reference))
  (|CallParentFunction OtherActor) ; This node is disabled and will not be called.\nDrag off pins to build functionality.
)

(event EventTick
  (params (DeltaSeconds :type Float%20%28single-precision%29))
  (|CallParentFunction DeltaSeconds) ; This node is disabled and will not be called.\nDrag off pins to build functionality.
)

(event EventToggleCombat
  (params (B_EnableCombat? :type Boolean))
  (|CallParentFunction B_EnableCombat?)
  (CallFunction|AttackOff-HandWeapon (select B_EnableCombat? (Variables|Socket|GetSecond%20Weapon%20Hand%20Socket) (Variables|Socket|GetSecond%20Weapon%20Attach%20Socket))))

(fn ConstructionScript
  (|CallParentFunction))

(fn ActivateCollision
  (params (CollisionPart :type E_CollisionPart%20Enum :default "NewEnumerator0"))
  (switch Utilities|FlowControl|Switch|SwitchonE_CollisionPart CollisionPart
    (:NewEnumerator0
      (Default|EnableCollision (Variables|Default|GetAC_CollisionComponent)))
    (:NewEnumerator1
      (Default|EnableCollision (Variables|Default|GetAC_CollisionComponent%20Left)))))

(fn DeactivateCollision
  (params (CollisionPart :type E_CollisionPart%20Enum :default "NewEnumerator0"))
  (switch Utilities|FlowControl|Switch|SwitchonE_CollisionPart CollisionPart
    (:NewEnumerator0
      (Default|DisableCollision (Variables|Default|GetAC_CollisionComponent)))
    (:NewEnumerator1
      (Default|DisableCollision (Variables|Default|GetAC_CollisionComponent%20Left)))))

(fn OnEquip
  (|CallParentFunction)
  (Default|SetCollisionMesh (Variables|Default|GetAC_CollisionComponent%20Left) (Variables|Default|GetOff-Hand))
  (CallFunction|AttackOff-HandWeapon (select (Default|GetCombatEnable (Variables|Default|GetRef_AC_CombatComponent)) (Variables|Socket|GetSecond%20Weapon%20Hand%20Socket) (Variables|Socket|GetSecond%20Weapon%20Attach%20Socket))))

(fn AttackOff-HandWeapon
  (params (Socket :type Name))
  (Development|PrintString (Utilities|String|ToString(Name) Socket))
  (Transformation|AttachComponentToComponent (Variables|Default|GetOff-Hand) (Variables|/Script/Engine.Character|GetMesh (.AsCharacter (Utilities|Casting|CastToCharacter (Components|GetOwner)))) Socket "SnapToTarget" "SnapToTarget" "SnapToTarget" true))