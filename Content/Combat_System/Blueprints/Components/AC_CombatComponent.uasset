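; Actor component that holds combat state for its owner: main weapon, combat-enabled flag, attack combo state and blocking.
; Setting a new main weapon unequips and destroys any existing one before storing the replacement.
; Combat toggles and blocking changes broadcast through event dispatchers, with blocking firing only when the value changes.
; ResetAttack clears the attack count and saved-attack flag; the component has no BeginPlay or Tick logic.
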(event EventBeginPlay)

(event EventTick
  (params (DeltaSeconds :type Float%20%28single-precision%29)))

(fn SetMainWeapon
  (params (NewWeapon :type BP%20Base%20Weapon%20Object%20Reference))
  (Utilities|FlowControl|Sequence
    (:then_0
      (Utilities|IsValid (Variables|Default|GetMainWeapon)
        (:Is%20Valid
          (Default|OnUnEquip (Variables|Default|GetMainWeapon))
          (Actor|DestroyActor (Variables|Default|GetMainWeapon)))))
    (:then_1
      (Variables|Default|SetMainWeapon NewWeapon))))

(fn GetMainWeapon
  (return (Variables|Default|GetMainWeapon)))

(fn SetCombatEnable
  (params (B_CombatEnable? :type Boolean))
  (bind _output_get (Variables|Default|SetB_CombatEnable? B_CombatEnable?))
  (Default|CallOnCombatToggled _output_get))

(fn GetCombatEnable
  (return (Variables|Default|GetB_CombatEnable?)))

(fn ResetAttack
  (Variables|Debug|SetAttackCount 0)
  (Variables|Debug|SetB_AttackSaved? false))

(fn SetBlockingState
  (params (Enable%20Blocking? :type Boolean))
  (if (!= Enable%20Blocking? (Variables|Debug|GetB_IsBlocking?))
    (bind _output_get (Variables|Debug|SetB_IsBlocking? Enable%20Blocking?))
    (Default|CallOnBlockingSet _output_get)))

(fn GetIsBlocking?
  (return (Variables|Debug|GetB_IsBlocking?)))