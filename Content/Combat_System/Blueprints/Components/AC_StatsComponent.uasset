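; Actor component for the combat system that stores character stats such as Health, Armor and Stamina.
; Base and max values seed a current-value map, whose changes are clamped on modify and broadcast through an update dispatcher.
; TakeDamage reduces damage by Armor and sets the owner's state manager to Death at zero Health.
; Stamina regenerates on a looping timer until full; the regeneration delay nodes are unconnected.
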(event Custom|StartRegeneration
  (params (Stat%20Type :type E_Stats%20Enum :default "NewEnumerator0"))
  (switch Utilities|FlowControl|Switch|SwitchonE_Stats Stat%20Type
    (:NewEnumerator2
      (Utilities|Time|SetTimerbyFunctionName 0 "RegenerationStamina" 0.1 true))))

(event EventBeginPlay)

(event EventTick
  (params (DeltaSeconds :type Float%20%28single-precision%29)))

(fn SetCurrentStatsValue
  (params (Stat :type E_Stats%20Enum :default "NewEnumerator0") (Value :type Float%20%28double-precision%29))
  (Utilities|Map|Add (Variables|Default|GetCurrentStats) Stat Value)
  (Default|CallOnCurrentStartValueUpdate Stat Value))

(fn GetCurrentStatsValue
  (params (Stat :type E_Stats%20Enum :default "NewEnumerator0"))
  (return (.Value (Utilities|Map|Find (Variables|Default|GetCurrentStats) Stat))))

(fn InitializeStats
  (bind _keys (Utilities|Map|Keys (Variables|BaseStats|GetBaseStats)))
  (for _array_element _keys
    (CallFunction|SetCurrentStatsValue _array_element (.basevalue (.Value (Utilities|Map|Find (Variables|BaseStats|GetBaseStats) _array_element))))))

(fn ModifyCurrentStatValue
  (params (Stat :type E_Stats%20Enum :default "NewEnumerator0") (Value :type Float%20%28double-precision%29) (B_ShouldStaminaRegeneration? :type Boolean))
  (if (!= Value 0.0)
    (bind _output_get (LocalVariables|SetL_SetValue (+ (CallFunction|GetCurrentStatsValue Stat) Value)))
    (bind _output_get_2 (LocalVariables|SetL_SetValue (Math|Float|Clamp(Float) _output_get 0.0 (BaseStats|GetMaxStatValue Stat))))
    (CallFunction|SetCurrentStatsValue Stat _output_get_2)
    (if B_ShouldStaminaRegeneration?
      (CallFunction|StartRegeneration Stat))))

(fn GetBaseStatValue
  (params (Stat :type E_Stats%20Enum :default "NewEnumerator0"))
  (return (.basevalue (.Value (Utilities|Map|Find (Variables|BaseStats|GetBaseStats) Stat)))))

(fn GetMaxStatValue
  (params (Stat :type E_Stats%20Enum :default "NewEnumerator0"))
  (return (.maxvalue (.Value (Utilities|Map|Find (Variables|BaseStats|GetBaseStats) Stat)))))

(fn SetBaseStatValue
  (params (Stat :type E_Stats%20Enum :default "NewEnumerator0") (Value :type Float%20%28double-precision%29))
  (Utilities|Struct|SetmembersinF_BaseStat (.Value (Utilities|Map|Find (Variables|BaseStats|GetBaseStats) Stat)) Value)
  (Utilities|Map|Add :TargetMap (Variables|BaseStats|GetBaseStats) :Key Stat))

(fn SetMaxStatValue
  (params (Stat :type E_Stats%20Enum :default "NewEnumerator0") (Value :type Float%20%28double-precision%29))
  (Utilities|Struct|SetmembersinF_BaseStat (.Value (Utilities|Map|Find (Variables|BaseStats|GetBaseStats) Stat)) Value)
  (Utilities|Map|Add :TargetMap (Variables|BaseStats|GetBaseStats) :Key Stat))

(fn TakeDamage
  (params (InDamage :type Float%20%28double-precision%29))
  (bind _value (CallFunction|GetCurrentStatsValue "NewEnumerator3"))
  (bind _returnvalue (+ InDamage _value))
  (bind _returnvalue_2 (/ InDamage _returnvalue))
  (bind _returnvalue_3 (* InDamage _returnvalue_2))
  (LocalVariables|SetL_SetDamage (Math|Float|Clamp(Float) _returnvalue_3 0.0 _returnvalue_3))
  (CallFunction|ModifyCurrentStatValue "NewEnumerator1" (* (LocalVariables|GetL_SetDamage) -1.0) true)
  (if (<= (CallFunction|GetCurrentStatsValue "NewEnumerator1") 0.0)
    (Default|SetCurrentState (Actor|GetComponentbyClass (Components|GetOwner) "/Game/Combat_System/Blueprints/Components/AC_StateManagerComponent.AC_StateManagerComponent_C") "(TagName=\"Character.State.Death\")")))

(fn RegenerationStamina
  (CallFunction|SetCurrentStatsValue "NewEnumerator2" (Math|Float|Clamp(Float) (+ (CallFunction|GetCurrentStatsValue "NewEnumerator2") (Variables|Stamina|GetStaminaRegenerationRate)) 0.0 (BaseStats|GetMaxStatValue "NewEnumerator2")))
  (if (>= (CallFunction|GetCurrentStatsValue "NewEnumerator2") (BaseStats|GetMaxStatValue "NewEnumerator2"))
    (Utilities|Time|ClearTimerbyFunctionName 0 "RegenerationStamina")))