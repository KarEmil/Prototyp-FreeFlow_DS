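; AC_CollisionComponent is a combat component that detects hits along a mesh, reporting each actor at most once per activation.
; While enabled, Tick runs a multi sphere trace for objects between start and end sockets on an assigned mesh component.
; CanHitActor rejects already-hit actors, ignored classes and actors with ignored gameplay tags; accepted hits are recorded and passed to OnHit.
; EnableCollision clears the hit list, starting a fresh detection window.
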(event Custom|EnableCollision
  (CallFunction|ClearHitActors)
  (Variables|Default|SetB_CollisionEnabled? true))

(event Custom|Disable%20Collision
  (Variables|Default|SetB_CollisionEnabled? false))

(event Custom|Collision%20Trace
  (bind _collisionmeshcomponent (Variables|Default|GetCollisionMeshComponent))
  (bind _outhits (Collision|MultiSphereTraceForObjects (Transformation|GetSocketLocation _collisionmeshcomponent (Variables|Initalization|GetStart%20Socket%20Name)) (Transformation|GetSocketLocation _collisionmeshcomponent (Variables|Initalization|GetEnd%20Socket%20Name)) (Variables|Initalization|GetTraceRadius) (Variables|Initalization|GetCollision%20Object%20Types) false (Variables|Default|GetActors%20to%20Ignore) (Variables|Initalization|GetDraw%20Debug%20Type)))
  (for _array_element _outhits
    (bind _output_get (Variables|Default|SetLastHit _array_element))
    (if (CallFunction|CanHitActor? (.HitActor (Collision|BreakHitResult _output_get)))
      (bind _output_get_2 (Variables|Default|SetHit%20Actor (.HitActor (Collision|BreakHitResult _output_get))))
      (Utilities|Array|Add (Variables|Default|GetAlredyHitActiors) _output_get_2)
      (Default|CallOnHit (Variables|Default|GetLastHit)))))

(event Custom|ClearHitActors
  (Utilities|Array|Clear (Variables|Default|GetAlredyHitActiors)))

(event Custom|SetCollisionMesh
  (params (CollisionMeshComponent :type Primitive%20Component%20Object%20Reference))
  (Variables|Default|SetCollisionMeshComponent CollisionMeshComponent))

(event EventBeginPlay)

(event EventTick
  (params (DeltaSeconds :type Float%20%28single-precision%29))
  (if (Variables|Default|GetB_CollisionEnabled?)
    (CallFunction|CollisionTrace)))

(fn GetAlredyHitActor
  (return (Variables|Default|GetAlredyHitActiors)))

(fn GetBCollisionEnabled?
  (return (Variables|Default|GetB_CollisionEnabled?)))

(fn GetLastHit
  (return (Variables|Default|GetLastHit)))

(fn GetCollisionMeshComponent
  (return (Variables|Default|GetCollisionMeshComponent)))

(fn AddActortoIgnore
  (params (InActor :type Actor%20Object%20Reference%20%28by%20ref%29))
  (Utilities|Array|AddUnique (Variables|Default|GetActors%20to%20Ignore) InActor))

(fn RemoveActortoIgnore
  (params (InActorRemove :type Actor%20Object%20Reference%20%28by%20ref%29))
  (Utilities|Array|RemoveItem (Variables|Default|GetActors%20to%20Ignore) InActorRemove))

(fn GetActortoIgnore
  (return (Variables|Default|GetActors%20to%20Ignore)))

(fn CanHitActor?
  (params (In%20Actor :type Actor%20Object%20Reference%20%28by%20ref%29))
  (bind _newparam (Class|BPIGameplayTagBlueprintTag|GetOwnedGameplayTag(Message) In%20Actor))
  (return (Math|Boolean|ANDBoolean (not (GameplayTags|HasAnyTags _newparam (Variables|Initalization|GetGameplayTagsToIgnore) true)) (not (Utilities|Array|ContainsItem (Variables|Default|GetAlredyHitActiors) In%20Actor)) (not (Utilities|Array|ContainsItem (Variables|Initalization|GetActorToIgnore) (Utilities|GetClass In%20Actor))))))