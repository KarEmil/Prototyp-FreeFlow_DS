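; Actor component that gives its owning character target lock-on, toggled on and off, in the combat system.
; Lock-on sphere-traces along the follow camera for a BPI_Targeting actor, and Tick interpolates control rotation toward it with clamped pitch.
; When the target dies or becomes untargetable, it switches to the nearest targetable actor found by sphere overlap.
; Character rotation switches between camera and movement orientation based on lock-on, combat state and movement speed mode.
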(event Custom|Next%20Lock%20On
  (CallFunction|SetBIsTargeting false)
  (bind (_returnvalue _foundtarget) (CallFunction|NextTarget))
  (if (and _returnvalue (CallFunction|CanTargetActor _foundtarget))
    (CallFunction|SetTargetActor _foundtarget)
    (CallFunction|SetBIsTargeting true)
    (CallFunction|UpdateRotationMode)))

(event Custom|Disable%20Lock%20On
  (CallFunction|SetBIsTargeting false)
  (CallFunction|SetTargetActor)
  (CallFunction|UpdateRotationMode))

(event Custom|ToggleLockOn
  (if (not (CallFunction|GetBIsTargeting))
    (CallFunction|EnableLockon)
    (else
      (CallFunction|DisableLockon))))

(event Custom|Enable%20Lock%20On
  (bind (_returnvalue _foundtarget) (CallFunction|FindTarget))
  (if (and _returnvalue (CallFunction|CanTargetActor _foundtarget))
    (CallFunction|SetTargetActor _foundtarget)
    (CallFunction|SetBIsTargeting true)
    (CallFunction|UpdateRotationMode)))

(event EventBeginPlay
  (bind _ascharacter (Utilities|Casting|CastToCharacter (Components|GetOwner)))
  (Variables|Components|SetOwnerCharacter _ascharacter)
  (Variables|Components|SetOwnerController (Pawn|GetController (Variables|Components|GetOwnerCharacter)))
  (Variables|Default|SetFollowCamera (Actor|GetComponentbyClass (Variables|Components|GetOwnerCharacter) "/Script/Engine.CameraComponent")))

(event EventTick
  (params (DeltaSeconds :type Float%20%28single-precision%29))
  (if (Variables|Default|GetB_IsTargering)
    (CallFunction|UpDateTargetControlRotation)))

(fn GetBIsTargeting
  (return (Variables|Default|GetB_IsTargering)))

(fn SetBIsTargeting
  (params (B_EnableTargering :type Boolean))
  (Variables|Default|SetB_IsTargering B_EnableTargering)
  (bind _targetactor (Variables|Default|GetTargetActor)
    (:then
      (Class|BPITargeting|OnTarget(Message) _targetactor B_EnableTargering))
    (:else)))

(fn FindTarget
  (bind (_outhit _returnvalue) (Collision|SphereTraceForObjects (Transformation|GetActorLocation (Components|GetOwner)) (+ (+ (* (Math|Vector|GetForwardVector (Variables|Default|GetFollowCamera)) (Variables|TargetInitialization|GetTargetingDistance)) (Transformation|GetActorLocation (Components|GetOwner))) (Math|Vector|MakeVector 0.0 0.0 (Variables|TargetInitialization|GetHighTargeting))) (Variables|TargetInitialization|GetTargetingRadius) (Variables|TargetInitialization|GetTargetObjectTypes) false (Utilities|Array|MakeArray (Components|GetOwner)) (Variables|Default|GetDraw%20Debug%20Type)))
  (if (and _returnvalue (Utilities|IsValid (.HitActor (Collision|BreakHitResult _outhit))))
    (if (Utilities|DoesObjectImplementInterface (.HitActor (Collision|BreakHitResult _outhit)) "/Game/Combat_System/Blueprints/Interface/BPI_Targeting.BPI_Targeting_C")
      (return true (.HitActor (Collision|BreakHitResult _outhit)))
      (else
        (return false 0)))
    (else
      (return false 0))))

(fn SetTargetActor
  (params (NewTargetActor :type Actor%20Object%20Reference))
  (Variables|Default|SetTargetActor NewTargetActor))

(fn GetTargetActor
  (return (Variables|Default|GetTargetActor)))

(fn UpDateTargetControlRotation
  (bind _returnvalue (Utilities|Time|GetWorldDeltaSeconds))
  (bind _returnvalue_2 (Components|GetOwner))
  (bind _ownercontroller (Variables|Components|GetOwnerController))
  (bind _targetactor (Variables|Default|GetTargetActor))
  (bind _targetlocationinterpspeed (Variables|TargetInitialization|GetTargetLocationInterpSpeed))
  (bind _targetactor_2 (Variables|Default|GetTargetActor))
  (bind _returnvalue_3 (Transformation|GetActorLocation _returnvalue_2))
  (bind _returnvalue_4 (Transformation|GetActorLocation _targetactor))
  (bind _returnvalue_5 (Transformation|GetActorRotation _ownercontroller))
  (bind _returnvalue_6 (- _returnvalue_4 "0.000000,0.000000,100.000000"))
  (bind _returnvalue_7 (Math|Rotator|FindLookatRotation _returnvalue_3 _returnvalue_6))
  (bind _returnvalue_8 (Math|Interpolation|RInterpTo _returnvalue_5 _returnvalue_7 _returnvalue _targetlocationinterpspeed))
  (if (and (Utilities|IsValid (Variables|Components|GetOwnerCharacter)) (Utilities|IsValid (Variables|Default|GetTargetActor)))
    (if (and (CallFunction|CanTargetActor _targetactor_2) (!= (Default|GetCurrentState (Actor|GetComponentbyClass _targetactor_2 "/Game/Combat_System/Blueprints/Components/AC_StateManagerComponent.AC_StateManagerComponent_C")) "(TagName=\"Character.State.Death\")"))
      (Pawn|SetControlRotation (Variables|Components|GetOwnerController) (Math|Rotator|MakeRotator (.Roll (Math|Rotator|BreakRotator _returnvalue_5)) (Math|Float|Clamp(Float) (.pitch _returnvalue_8) -25.0 3e+01) (.yaw _returnvalue_8)))
      (else
        (CallFunction|DisableLockon)
        (CallFunction|NextLockon)))))

(fn SetRotationMode
  (params (NewRotation :type E_RotationMode%20Enum :default "NewEnumerator0"))
  (bind _ownercharacter (Variables|Components|GetOwnerCharacter))
  (bind _charactermovement (Variables|/Script/Engine.Character|GetCharacterMovement _ownercharacter))
  (bind _output_get (Variables|Default|SetCurrentRotationMode NewRotation))
  (switch Utilities|FlowControl|Switch|SwitchonE_RotationMode _output_get
    (:NewEnumerator0
      (Variables|/Script/Engine.Pawn|SetbUseControllerRotationYaw _ownercharacter false)
      (Variables|/Script/Engine.CharacterMovementComponent|SetbUseControllerDesiredRotation _charactermovement true)
      (Variables|/Script/Engine.CharacterMovementComponent|SetbOrientRotationToMovement _charactermovement false))
    (:NewEnumerator1
      (Variables|/Script/Engine.Pawn|SetbUseControllerRotationYaw _ownercharacter false)
      (Variables|/Script/Engine.CharacterMovementComponent|SetbUseControllerDesiredRotation _charactermovement false)
      (Variables|/Script/Engine.CharacterMovementComponent|SetbOrientRotationToMovement _charactermovement true))))

(fn GetRotationMode
  (return (Variables|Default|GetCurrentRotationMode)))

(fn CanTargetActor
  (params (InTargetActor :type Actor%20Object%20Reference))
  (Utilities|IsValid InTargetActor
    (:Is%20Valid
      (bind _returnvalue (Class|BPITargeting|CanbeTargeted?(Message) InTargetActor))
      (return (and _returnvalue (< (Transformation|GetDistanceTo (Components|GetOwner) (Variables|Default|GetTargetActor)) (Variables|TargetInitialization|GetTargetingDistance)))))
    (:Is%20Not%20Valid
      (return false))))

(fn UpdateRotationMode
  (Utilities|IsValid (Variables|Default|GetOwnerCombatComponent)
    (:Is%20Valid
      _)
    (:Is%20Not%20Valid
      (Variables|Default|SetOwnerCombatComponent (Actor|GetComponentbyClass (Variables|Components|GetOwnerCharacter) "/Game/Combat_System/Blueprints/Components/AC_CombatComponent.AC_CombatComponent_C"))))
  (bind _returnvalue (Class|BPICombat|GetMovmentSpeedMode(Message) (Variables|Components|GetOwnerCharacter)))
  (CallFunction|SetRotationMode (select (Math|Boolean|ANDBoolean (Utilities|Enum|NotEqual(Enum) _returnvalue "NewEnumerator2") (Default|GetCombatEnable (Variables|Default|GetOwnerCombatComponent)) (CallFunction|GetBIsTargeting)) "NewEnumerator0" (Variables|TargetInitialization|GetDefaultRotationMode))))

(fn NextTarget
  (bind _targetactor (Variables|Default|GetTargetActor))
  (LocalVariables|SetL_DistanceFromTarget 0.0)
  (bind _output_get (LocalVariables|SetL_PlayerLocation (Transformation|GetActorLocation (Components|GetOwner))))
  (bind (_outactors _returnvalue) (Collision|SphereOverlapActors _output_get (Variables|TargetInitialization|GetNextTargetRadius) (Variables|TargetInitialization|GetTargetObjectTypes) 0 (Utilities|Array|MakeArray (Components|GetOwner) _targetactor)))
  (if _returnvalue
    (LocalVariables|SetL_DistanceFromTarget (Variables|TargetInitialization|GetNextTargetRadius))
    (for (_array_element _array_index) _outactors
      (bind _returnvalue_2 (Class|BPITargeting|CanbeTargeted?(Message) _array_element))
      (if (and _returnvalue_2 (< (Math|Vector|Distance(Vector) (Transformation|GetActorLocation _array_element) (LocalVariables|GetL_PlayerLocation)) (LocalVariables|GetL_DistanceFromTarget)))
        (LocalVariables|SetL_DistanceFromTarget (Math|Vector|Distance(Vector) (Transformation|GetActorLocation _array_element) (LocalVariables|GetL_PlayerLocation)))
        (LocalVariables|SetL_index _array_index)
        (LocalVariables|SetFindTarget true)))
    (if (LocalVariables|GetFindTarget)
      (return true (Utilities|Array|Get(acopy) _outactors (LocalVariables|GetL_index)))
      (else
        (LocalVariables|SetFindTarget false)
        (return false 0)))
    (else
      (return true _targetactor))))